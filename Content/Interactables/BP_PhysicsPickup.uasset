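; BP_PhysicsPickup is an interactable physics object that the player can pick up and drop.
; IntInteract runs only if the player holds nothing: it sets IsHolding, disables the Cube's physics and collision, and snaps it to the player's Arrow1, keeping relative rotation and scale.
; IntDrop detaches the actor in world space and restores collision and physics, but does not clear IsHolding.
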(event EventBeginPlay)

(event Collision|EventActorBeginOverlap
  (params (OtherActor :type Actor%20Object%20Reference)))

(event EventTick
  (params (DeltaSeconds :type Float%20%28single-precision%29)))

(event EventIntInteract
  (params (PlayerRef :type BP%20Player%20Char%20Object%20Reference))
  (bind _cube (Variables|Default|GetCube))
  (if (not (Variables|/Game/Player/BP_PlayerChar.BP_PlayerChar_C|GetisHolding? PlayerRef))
    (Variables|/Game/Player/BP_PlayerChar.BP_PlayerChar_C|SetisHolding? PlayerRef true)
    (Physics|SetSimulatePhysics _cube false)
    (Collision|SetCollisionEnabled _cube "NoCollision")
    (Transformation|AttachComponentToComponent (Variables|Default|GetCube) (Variables|/Game/Player/BP_PlayerChar.BP_PlayerChar_C|GetArrow1 PlayerRef) "None" "SnapToTarget" "KeepRelative" "KeepRelative" true)))

(event EventIntDrop
  (bind _cube (Variables|Default|GetCube))
  (Transformation|DetachFromActor "KeepWorld" "KeepWorld" "KeepWorld")
  (Collision|SetCollisionEnabled _cube "QueryAndPhysics")
  (Physics|SetSimulatePhysics _cube true))

(fn ConstructionScript)